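; BP_Pickup_SafeBox is a safe box pickup that spins in place until the player's car collects it.
; Tick plays a timeline whose track sets the Safe's world yaw and the negated yaw of StaticMesh1, while StaticMesh keeps its current rotation.
; When a NewCar overlaps the Sphere, it disables Safe collision, calls CollectSafeBox on the car and destroys itself.
; Other overlaps and hits only print debug messages.
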(event `self.ReceiveTick`
  (params (DeltaSeconds :type "Float (single-precision)"))
  (bind _safe (`self.Safe`))
  (bind (_returnvalue_roll _returnvalue_pitch) (`KismetMathLibrary.BreakRotator` (`SceneComponent.K2_GetComponentRotation` (`self.StaticMesh1`))))
  (bind (_returnvalue_roll_2 _returnvalue_pitch_2 _returnvalue_yaw) (`KismetMathLibrary.BreakRotator` (`SceneComponent.K2_GetComponentRotation` (`self.StaticMesh`))))
  (bind (_returnvalue_roll_3 _returnvalue_pitch_3) (`KismetMathLibrary.BreakRotator` (`SceneComponent.K2_GetComponentRotation` _safe)))
  ;[1 1 1] Rotation
  (bind (_direction _newtrack_0) (`Timeline|Timeline_0`)
    (:`Update`
      (`SceneComponent.K2_SetWorldRotation` _safe (`KismetMathLibrary.MakeRotator` _returnvalue_roll_3 _returnvalue_pitch_3 _newtrack_0) false false)
      (`SceneComponent.K2_SetWorldRotation` (`self.StaticMesh`) (`KismetMathLibrary.MakeRotator` _returnvalue_roll_2 _returnvalue_pitch_2 _returnvalue_yaw) false false)
      (`SceneComponent.K2_SetWorldRotation` (`self.StaticMesh1`) (`KismetMathLibrary.MakeRotator` _returnvalue_roll _returnvalue_pitch (- 0.0 _newtrack_0)) false false))))

(event `self.Sphere.OnComponentBeginOverlap`
  (params (OverlappedComponent :type "PrimitiveComponent Object Reference") (OtherActor :type "Actor Object Reference") (OtherComp :type "PrimitiveComponent Object Reference") (OtherBodyIndex :type Integer) (bFromSweep :type Boolean) (SweepResult :type "HitResult Structure (by ref)"))
  ;[1 1 1] Being Picked Up
  (`KismetSystemLibrary.PrintString` "Collision Detected!" false)
  (bind _asnew_car (cast `/Game/VehicleBPs/NewCar` OtherActor)
    (:`then`
      (`KismetSystemLibrary.PrintString` "PlayerCar hits a safe box!")
      (`PrimitiveComponent.SetCollisionEnabled` (`self.Safe`) "NoCollision")
      (`/Game/VehicleBPs/NewCar.CollectSafeBox` _asnew_car)
      (`self.K2_DestroyActor`))
    (:`CastFailed`
      (`KismetSystemLibrary.PrintString` "Something other than PlayerCar hits a safe box!"))))

(event `self.Sphere.OnComponentHit`
  (params (HitComponent :type "PrimitiveComponent Object Reference") (OtherActor :type "Actor Object Reference") (OtherComp :type "PrimitiveComponent Object Reference") (NormalImpulse :type "Vector Structure") (Hit :type "HitResult Structure (by ref)"))
  ;[1 1 1] Being Picked Up
  (`KismetSystemLibrary.PrintString` "Hit Detected!" false))

(fn `UserConstructionScript`)