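; PlayHUD manages the in-game widgets for the car's fuel level, safe-box count and Twitch user messages.
; On BeginPlay it shows a state widget for three seconds alongside the main UI, then swaps in the Twitch widget.
; UI updates read values from the NewCar actor, while Twitch updates show the passed message briefly.
; Both updates destroy and recreate their widget instead of refreshing it in place.
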(event `self.ReceiveBeginPlay`
  ;[1 1 1] Render UI at BeginPlay
  (bind _returnvalue (`|CreateWidget` "/Game/Blueprints/BP_State.BP_State_C" (`GameplayStatics.GetPlayerController` 0)))
  (bind _output_get (set `self.BP_State_Reference` _returnvalue))
  (`UserWidget.AddToViewport` _output_get 0)
  (bind _returnvalue_2 (`|CreateWidget` "/Game/Blueprints/BP_UI.BP_UI_C" (`GameplayStatics.GetPlayerController` 0)))
  (bind _output_get_2 (set `self.BP_UI_Reference` _returnvalue_2))
  (`UserWidget.AddToViewport` _output_get_2 0)
  (`self.Update_UI`)
  (`KismetSystemLibrary.Delay` 3.0)
  (`Widget.RemoveFromParent` (`self.BP_State_Reference`))
  (bind _returnvalue_3 (`|CreateWidget` "/Game/Blueprints/BP_Twitch.BP_Twitch_C" (`GameplayStatics.GetPlayerController` 0)))
  (bind _output_get_3 (set `self.BP_Twitch_Reference` _returnvalue_3))
  (`UserWidget.AddToViewport` _output_get_3 0))

(event `Update_UI`
  ;[1 1 1] Render UI when necessary
  (`KismetSystemLibrary.PrintString` "Update UI Display" false)
  (bind _returnvalue (`GameplayStatics.GetActorOfClass` "/Game/VehicleBPs/NewCar.NewCar_C"))
  (`Widget.RemoveFromParent` (`self.BP_UI_Reference`))
  (bind _returnvalue_2 (`|CreateWidget` "/Game/Blueprints/BP_UI.BP_UI_C" (`GameplayStatics.GetPlayerController` 0)))
  (set `self.BP_UI_Reference` _returnvalue_2)
  (set `/Game/Blueprints/BP_UI.PercentFuel` (/ (`KismetMathLibrary.Conv_IntToDouble` (`/Game/VehicleBPs/NewCar.Fuel_Current` _returnvalue)) 100.0) (`self.BP_UI_Reference`))
  (set `/Game/Blueprints/BP_UI.StrSafeNum` (`KismetStringLibrary.BuildString_Int` "" "" (`/Game/VehicleBPs/NewCar.Cnt_SafeBox` _returnvalue)) (`self.BP_UI_Reference`))
  (`UserWidget.AddToViewport` (`self.BP_UI_Reference`) 0))

(event `Update_Twitch`
  (params (TwitchUserMessage :type String))
  ;[1 1 1] Render UI when necessary
  (`Widget.RemoveFromParent` (`self.BP_Twitch_Reference`))
  (bind _returnvalue (`|CreateWidget` "/Game/Blueprints/BP_Twitch.BP_Twitch_C" (`GameplayStatics.GetPlayerController` 0)))
  (bind _output_get (set `self.BP_Twitch_Reference` _returnvalue))
  (set `/Game/Blueprints/BP_Twitch.VarString` TwitchUserMessage _output_get)
  (`UserWidget.AddToViewport` _output_get 0)
  (`KismetSystemLibrary.Delay` 2.0)
  (`Widget.RemoveFromParent` (`self.BP_Twitch_Reference`)))

(fn `UserConstructionScript`)